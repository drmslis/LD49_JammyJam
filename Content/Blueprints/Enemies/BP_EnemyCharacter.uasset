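; BP_EnemyCharacter is an enemy character that carries a sword through a child actor component.
; On BeginPlay it sets itself as the sword's owner, reuses BP_PlayerSwordWeapon by casting to it, switches the weapon collider to an overlap-all profile and sets its damage.
; Incoming damage is only printed for debugging; no health or death logic appears here.
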(event `self.ReceiveBeginPlay`
  (bind _childactor (`ChildActorComponent.ChildActor` (`self.ChildActor`)))
  (`self.SetOwner` _childactor self)
  (bind _asbp_player_sword_weapon (cast `/Game/Blueprints/Player/BP_PlayerSwordWeapon` _childactor))
  (`PrimitiveComponent.SetCollisionProfileName` (`/Game/Blueprints/Player/BP_BaseSwordWeapon.WeaponCollider` _asbp_player_sword_weapon) "OverlapAll" true)
  (set `/Game/Blueprints/Player/BP_BaseSwordWeapon.Damage` 30.0 _asbp_player_sword_weapon))

(event `self.ReceiveAnyDamage`
  (params (Damage :type "Float (single-precision)") (DamageType :type "DamageType Object Reference") (InstigatedBy :type "Controller Object Reference") (DamageCauser :type "Actor Object Reference"))
  (`KismetSystemLibrary.PrintString` (`KismetStringLibrary.Conv_DoubleToString` Damage)))

(fn `UserConstructionScript`)