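; BP_Leshiy is a boss-style enemy that attacks the player in range and switches streamed levels on death.
; An overlap sphere opens and closes a Tick gate that turns the capsule toward the player and loops random montages, throttled by a DoOnce.
; BeginPlay readies a child-actor sword's collider and plays a taunt.
; Damage triggers hit reactions until death locks attacks, loads SuperFinalMap4432 and unloads DevMap_beta.
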(event `self.ReceiveBeginPlay`
  (bind _childactor (`ChildActorComponent.ChildActor` (`self.ChildActor`)))
  (`self.SetOwner` _childactor self)
  (bind _asbp_leshiyr_sword_weapon_1 (cast `/Game/Blueprints/Player/BP_LeshiyrSwordWeapon1` _childactor))
  (`PrimitiveComponent.SetCollisionProfileName` (`/Game/Blueprints/Player/BP_BaseSwordWeapon.WeaponCollider` _asbp_leshiyr_sword_weapon_1) "OverlapAll" true)
  (set `self.CurrentHealth` (`self.MaxHealth`))
  (`GameplayStatics.PlaySoundAtLocation` (`self.SpawnSound`) (`self.K2_GetActorLocation`) (struct) 1.0 1.0 0.0 null null null)
  (`|PlayMontage` (`self.Mesh`) "/Game/Assets/Animations/Swordsman/Taunt/A_SW_Taunt_02_Montage.A_SW_Taunt_02_Montage" 0.6))

(event `self.ReceiveAnyDamage`
  (params (Damage :type "Float (single-precision)") (DamageType :type "DamageType Object Reference") (InstigatedBy :type "Controller Object Reference") (DamageCauser :type "Actor Object Reference"))
  (bind _mesh (`self.Mesh`))
  (set `self.CurrentHealth` (- (`self.CurrentHealth`) Damage))
  (if (> (`self.CurrentHealth`) 0.0)
    (`GameplayStatics.PlaySoundAtLocation` (`self.HitSound`) (`self.K2_GetActorLocation`) (struct) 1.0 1.0 0.0 null null null)
    ;[1 1 1] Get damage
    (`|PlayMontage` (`self.Mesh`) "/Game/Assets/Animations/BossyEnemy/Animations/Boss_ReactionHit_F_Montage.Boss_ReactionHit_F_Montage" 1.5)
    (else
      (`GameplayStatics.PlaySoundAtLocation` (`self.SpawnSound`) (`self.K2_GetActorLocation`) (struct) 1.0 1.0 0.0 null null null)
      ;[1 1 1] Death
      (`SkeletalMeshComponent.SetPlayRate` _mesh 0.5)
      (`SkeletalMeshComponent.PlayAnimation` _mesh "/Game/Assets/Animations/AnimStarterPack/Death_2.Death_2" false)
      (`self.AttackLock`)
      (set `self.IsDead` true)
      (`GameplayStatics.LoadStreamLevelBySoftObjectPtr` "/Game/Maps/StreamingLevels/SuperFinalMap4432.SuperFinalMap4432" true)
      (`GameplayStatics.UnloadStreamLevel` "DevMap_beta"))))

(event `self.ReceiveTick`
  (params (DeltaSeconds :type "Float (single-precision)"))
  (`/Engine/EditorBlueprintResources/StandardMacros.Gate` true :!label _label
    (:`Exit`
      (`SceneComponent.K2_SetWorldRotation` (`self.CapsuleComponent`) (`KismetMathLibrary.FindLookAtRotation` (`SceneComponent.K2_GetComponentLocation` (`self.CapsuleComponent`)) (`SceneComponent.K2_GetComponentLocation` (`Character.CapsuleComponent` (`self.As BP Player`)))) false false)
      (`/Engine/EditorBlueprintResources/StandardMacros.DoOnce` false :!label _label_2
        (:`Completed`
          (switch `int` (`KismetMathLibrary.RandomIntegerInRange` 0 2)
            (:`0`
              (`|PlayMontage` (`self.Mesh`) "/Game/Assets/Animations/BossyEnemy/Animations/Boss_ReactionHit_F_Montage.Boss_ReactionHit_F_Montage"
                (:`OnCompleted`
                  (`KismetSystemLibrary.Delay` 0.2)
                  (goto _label_2 :!via `Reset`))
                (:`OnInterrupted`
                  (goto _label_2 :!via `Reset`))))
            (:`1`
              (`|PlayMontage` (`self.Mesh`) "/Game/Assets/Animations/BossyEnemy/Animations/InPlace/Attacks/Boss_Attack_Uppercut_InP_Montage.Boss_Attack_Uppercut_InP_Montage"
                (:`OnCompleted`
                  (`KismetSystemLibrary.Delay` 0.2)
                  (goto _label_2 :!via `Reset`))
                (:`OnInterrupted`
                  (goto _label_2 :!via `Reset`))))
            (:`2`
              (`|PlayMontage` (`self.Mesh`) "/Game/Assets/Animations/BossyEnemy/Animations/InPlace/Attacks/Boss_Attack_Swing_InP_Montage.Boss_Attack_Swing_InP_Montage"
                (:`OnCompleted`
                  (`KismetSystemLibrary.Delay` 0.2)
                  (goto _label_2 :!via `Reset`))
                (:`OnInterrupted`
                  (goto _label_2 :!via `Reset`))))))))))

(event `AttackUnlock`
  (goto _label :!via `Open`))

(event `AttackLock`
  (goto _label :!via `Close`))

(event `self.Sphere.OnComponentBeginOverlap`
  (params (OverlappedComponent :type "PrimitiveComponent Object Reference") (OtherActor :type "Actor Object Reference") (OtherComp :type "PrimitiveComponent Object Reference") (OtherBodyIndex :type Integer) (bFromSweep :type Boolean) (SweepResult :type "HitResult Structure (by ref)"))
  (bind _asbp_player (cast `/Game/Blueprints/Player/BP_Player` OtherActor))
  (set `self.As BP Player` _asbp_player)
  (if (not (`self.IsDead`))
    (`self.AttackUnlock`)))

(event `self.Sphere.OnComponentEndOverlap`
  (params (OverlappedComponent :type "PrimitiveComponent Object Reference") (OtherActor :type "Actor Object Reference") (OtherComp :type "PrimitiveComponent Object Reference") (OtherBodyIndex :type Integer))
  (cast `/Game/Blueprints/Player/BP_Player` OtherActor)
  (`self.AttackLock`))

(fn `UserConstructionScript`)