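; StreamingTrigger is a trigger volume that streams in the next level as an instance when BP_Player overlaps its box.
; The level loads at a stored zero point plus X/Y map offsets, only while no valid loaded level is held.
; It then passes itself to BP_TestGamemode via RequestLevelUpdate.
; GetZeroPoint stores the supplied origin, and Invalidate clears the level reference so the trigger can load again.
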(event `self.Box.OnComponentBeginOverlap`
  (params (OverlappedComponent :type "PrimitiveComponent Object Reference") (OtherActor :type "Actor Object Reference") (OtherComp :type "PrimitiveComponent Object Reference") (OtherBodyIndex :type Integer) (bFromSweep :type Boolean) (SweepResult :type "HitResult Structure (by ref)"))
  (bind (_zeropointlocation_x _zeropointlocation_y) (`KismetMathLibrary.BreakVector` (`self.ZeroPointLocation`)))
  (cast `/Game/Blueprints/Player/BP_Player` OtherActor)
  (`/Engine/EditorBlueprintResources/StandardMacros.IsValid` (`self.LoadedLevel`)
    (:`Is Not Valid`
      (bind (_boutsuccess _returnvalue) (`LevelStreamingDynamic.LoadLevelInstanceBySoftObjectPtr` "/Game/Maps/StreamingLevels/LevelNext.LevelNext" (`KismetMathLibrary.MakeVector` (+ _zeropointlocation_x (`self.X_Map_offset`)) (+ _zeropointlocation_y (`self.Y_Map_offset`))) (`self.Rotation`)))
      (set `self.LoadedLevel` _returnvalue)
      (bind _asbp_test_gamemode (cast `/Game/Blueprints/Gamemode/BP_TestGamemode` (`GameplayStatics.GetGameMode`)))
      (`/Game/Blueprints/Gamemode/BP_TestGamemode.RequestLevelUpdate` _asbp_test_gamemode self))))

(event `self.ReceiveTick`
  (params (DeltaSeconds :type "Float (single-precision)")))

(event `Invalidate`
  (set `self.LoadedLevel` null))

(event `GetZeroPoint`
  (params (ZeroPointLocation :type "Vector Structure") (ZeroPointRotation :type "Rotator Structure"))
  (set `self.ZeroPointLocation` ZeroPointLocation)
  (set `self.ZeroPointRotation` ZeroPointRotation))

(fn `UserConstructionScript`)