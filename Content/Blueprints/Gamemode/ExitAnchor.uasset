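; Exit trigger actor that streams exit rooms in and out for a ForestManager as the player moves through it.
; Entering MainBox has the manager spawn exit rooms once; backing out unloads them and re-arms the spawn.
; Flags from overlapping MainBox and LeaveBox give crossing direction: exiting LeaveBox outside MainBox activates the next manager and unloads the current manager's level.
; Debug prints trace each transition.
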(event `self.MainBox.OnComponentBeginOverlap`
  (params (OverlappedComponent :type "PrimitiveComponent Object Reference") (OtherActor :type "Actor Object Reference") (OtherComp :type "PrimitiveComponent Object Reference") (OtherBodyIndex :type Integer) (bFromSweep :type Boolean) (SweepResult :type "HitResult Structure (by ref)"))
  (if (`KismetSystemLibrary.IsValid` (`self.ForestManager`))
    (if (== OtherActor (cast `/Game/Blueprints/Player/BP_Player` OtherActor :!pure true))
      (set `self.A` true)
      (`KismetSystemLibrary.PrintString` "Enter A" true true (struct :`G` 0.66 :`B` 1.0 :`A` 1.0) 4.0)
      (if (not (`self.Already Loaded?`))
        (`/Game/Blueprints/Gamemode/ForestManager.SpawnExitRooms` (`self.ForestManager`) self)
        (set `self.Already Loaded?` true)))))

(event `UnlockSelfDestruction`
  (`/Engine/EditorBlueprintResources/StandardMacros.Gate` false :!via `Open` :!label _label))

(event `BlockSelfDestruction`
  (goto _label :!via `Close`))

(event `self.MainBox.OnComponentEndOverlap`
  (params (OverlappedComponent :type "PrimitiveComponent Object Reference") (OtherActor :type "Actor Object Reference") (OtherComp :type "PrimitiveComponent Object Reference") (OtherBodyIndex :type Integer))
  (bind _loadedlevel (`/Game/Blueprints/Gamemode/ForestManager.LoadedLevel` (`self.ForestManager`)))
  (if (`.bSuccess` (cast `/Game/Blueprints/Player/BP_Player` OtherActor :!pure true))
    (if (`KismetSystemLibrary.IsValid` _loadedlevel)
      (set `self.A` false)
      (if (`self.B`)
        (`KismetSystemLibrary.PrintString` "Prepare to leave" true true (struct :`G` 0.66 :`B` 1.0 :`A` 1.0) 4.0)
        (else
          (set `self.A` false)
          (`LevelStreaming.SetIsRequestingUnloadAndRemoval` _loadedlevel true)
          (`KismetSystemLibrary.PrintString` "Unload Loaded" true true (struct :`G` 0.66 :`B` 1.0 :`A` 1.0) 4.0)
          (set `self.Already Loaded?` false))))))

(event `self.LeaveBox.OnComponentBeginOverlap`
  (params (OverlappedComponent :type "PrimitiveComponent Object Reference") (OtherActor :type "Actor Object Reference") (OtherComp :type "PrimitiveComponent Object Reference") (OtherBodyIndex :type Integer) (bFromSweep :type Boolean) (SweepResult :type "HitResult Structure (by ref)"))
  (if (`.bSuccess` (cast `/Game/Blueprints/Player/BP_Player` OtherActor :!pure true))
    (set `self.B` true)
    (`KismetSystemLibrary.PrintString` "Enter B" true true (struct :`G` 0.66 :`B` 1.0 :`A` 1.0) 4.0)))

(event `self.LeaveBox.OnComponentEndOverlap`
  (params (OverlappedComponent :type "PrimitiveComponent Object Reference") (OtherActor :type "Actor Object Reference") (OtherComp :type "PrimitiveComponent Object Reference") (OtherBodyIndex :type Integer))
  (bind _forestmanager (`self.ForestManager`))
  (if (`.bSuccess` (cast `/Game/Blueprints/Player/BP_Player` OtherActor :!pure true))
    (set `self.B` false)
    (if (`self.A`)
      (`KismetSystemLibrary.PrintString` "Stay")
      (else
        (`KismetSystemLibrary.PrintString` "Leave")
        (`/Game/Blueprints/Gamemode/ForestManager.ActivateNextManager` _forestmanager)
        (`LevelStreaming.SetIsRequestingUnloadAndRemoval` (`/Game/Blueprints/Gamemode/ForestManager.SelfLevel` _forestmanager) true)))))

(event `self.ReceiveTick`
  (params (DeltaSeconds :type "Float (single-precision)")))

(fn `UserConstructionScript`)