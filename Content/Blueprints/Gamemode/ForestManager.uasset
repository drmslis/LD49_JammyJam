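; Forest room manager actor that registers with BP_TestGamemode and streams in the next level from an exit trigger.
; It passes the trigger's transform to the streamed level so its entrance can align to that exit.
; It hands level history to the newest registered manager and can activate that manager's backtrack overlap boxes.
; Level-instance loading, unloading and compensation calls are disconnected, and debug prints remain, including one every Tick.
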(event `self.ReceiveBeginPlay`
  (bind _asbp_test_gamemode (cast `/Game/Blueprints/Gamemode/BP_TestGamemode` (`GameplayStatics.GetGameMode`)))
  (`/Game/Blueprints/Gamemode/BP_TestGamemode.AddForestManager` _asbp_test_gamemode self))

(event `EntranceToExit`
  (params (NewTransform :type "Transform Structure (by ref)"))
  (if (`KismetSystemLibrary.IsValid` (`self.EntranceAnchor`))
    (if (`self.HasAlignedEntranceToExit`)
      (`self.K2_SetActorTransform` (`self.EntranceAnchor`) NewTransform false false)
      (set `self.HasAlignedEntranceToExit` true))))

(event `SpawnExitRooms`
  (params (ActivatedTrigger :type "/Game/Blueprints/Gamemode/ExitAnchor Object Reference"))
  (bind (_returnvalue_location _returnvalue_rotation) (`KismetMathLibrary.BreakTransform` (`self.GetTransform` (`self.ActivatedTrigger`))))
  (`KismetSystemLibrary.PrintString` "Hello")
  (if (`KismetSystemLibrary.IsValid` (`self.ActivatedTrigger`))
    (set `self.ActivatedTrigger` ActivatedTrigger)
    (else
      (set `self.ActivatedTrigger` ActivatedTrigger)))
  (`GameplayStatics.LoadStreamLevel` (`self.Next Level Name`) true)
  (message `/Game/Data/LevelScripts.AlignEntranceToExit` (`GameplayStatics.GetStreamingLevel` (`self.Next Level Name`)) (`KismetMathLibrary.MakeTransform` _returnvalue_location _returnvalue_rotation) "None"))

(event `ActivateCompensation`
  (params (Rotator :type "Rotator Structure"))
  (set `self.Rotator` Rotator))

(event `self.ReceiveTick`
  (params (DeltaSeconds :type "Float (single-precision)"))
  (`KismetSystemLibrary.PrintString` (`KismetStringLibrary.Conv_RotatorToString` (`KismetMathLibrary.MakeRotFromX` (`self.GetActorForwardVector`))) true true (struct :`G` 0.66 :`B` 1.0 :`A` 1.0) 0.0))

(event `GetNewManager`
  (bind _asbp_test_gamemode (cast `/Game/Blueprints/Gamemode/BP_TestGamemode` (`GameplayStatics.GetGameMode`)))
  (bind _forestmanagers (`/Game/Blueprints/Gamemode/BP_TestGamemode.ForestManagers` _asbp_test_gamemode))
  (bind _output (`|GetArrayItem` _forestmanagers (`KismetArrayLibrary.Array_LastIndex` _forestmanagers)))
  (`self.SetLevelComeFrom` _output (`self.SelfLevel`))
  (`self.SetSelfLevel` _output (`self.LoadedLevel`)))

(event `SetSelfLevel`
  (params (SelfLevel :type "LevelStreamingDynamic Object Reference"))
  (set `self.SelfLevel` SelfLevel))

(event `SetLevelComeFrom`
  (params (`LevelWeCame From` :type "LevelStreamingDynamic Object Reference"))
  (set `self.LevelWeCame From` `LevelWeCame From`))

(event `ReadyToUnloadStart`
  (if (not (== (`self.CurrentLocationName`) "FirstMap"))
    (bind _asbp_test_gamemode (cast `/Game/Blueprints/Gamemode/BP_TestGamemode` (`GameplayStatics.GetGameMode`)))
    (`/Game/Blueprints/Gamemode/BP_TestGamemode.Unlock` _asbp_test_gamemode)))

(event `ActivateNextManager`
  (bind _asbp_test_gamemode (cast `/Game/Blueprints/Gamemode/BP_TestGamemode` (`GameplayStatics.GetGameMode`)))
  (bind _forestmanagers (`/Game/Blueprints/Gamemode/BP_TestGamemode.ForestManagers` _asbp_test_gamemode))
  (bind _output (`|GetArrayItem` _forestmanagers (`KismetArrayLibrary.Array_LastIndex` _forestmanagers)))
  (set `/Game/Blueprints/Gamemode/ForestManager.IsActive` true _output)
  (`self.ActivateBackTrack` _output)
  (`self.SetLevelComeFrom` _output (`self.SelfLevel`))
  (`self.SetSelfLevel` _output (`self.LoadedLevel`)))

(event `ActivateBackTrack`
  (bind _output (`|GetArrayItem` (`self.ExitAnchors`) 6))
  (if (`self.IsActive`)
    (set `PrimitiveComponent.bGenerateOverlapEvents` true (`/Game/Blueprints/Gamemode/ExitAnchor.LeaveBox` _output))
    (set `PrimitiveComponent.bGenerateOverlapEvents` true (`/Game/Blueprints/Gamemode/ExitAnchor.MainBox` _output))))

(fn `Positive`
  (params (NewParam :type "Float (double-precision)"))
  (returns (NewParam1 :type "Float (double-precision)"))
  (if (>= NewParam 0.0)
    (return NewParam)
    (else
      (return (* NewParam -1.0)))))

(fn `UserConstructionScript`)

(fn `WhichMapToSpawn`
  (returns (MapToSpawn :type Name))
  (return (`|GetArrayItem` (`self.SpawnableRooms`) (`self.LoadingLevelsLoopCount`))))