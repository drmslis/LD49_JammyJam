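; Test game mode that manages streamed levels and respawns the player's pawn on BeginPlay.
; AddLevel tracks streamed levels and, beyond three, unloads the oldest, also unloading FirstMap through a gate that Unlock opens.
; RequestLevelUpdate stores a trigger if none is current; otherwise it unloads and invalidates the current one and clears it.
; It also collects forest managers; CreateNewLevel is an empty stub.
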(event `CreateNewLevel`)

(event `RequestLevelUpdate`
  (params (TrigerRequest :type "/Game/Blueprints/Gamemode/StreamingTrigger Object Reference"))
  (`/Engine/EditorBlueprintResources/StandardMacros.IsValid` (`self.CurrentTriger`)
    (:`Is Valid`
      (`LevelStreaming.SetIsRequestingUnloadAndRemoval` (`/Game/Blueprints/Gamemode/StreamingTrigger.LoadedLevel` (`self.CurrentTriger`)) true)
      (`/Game/Blueprints/Gamemode/StreamingTrigger.Invalidate` (`self.CurrentTriger`))
      (set `self.CurrentTriger` null))
    (:`Is Not Valid`
      (set `self.CurrentTriger` TrigerRequest))))

(event `AddLevel`
  (params (NewLevel :type "LevelStreamingDynamic Object Reference"))
  (`KismetArrayLibrary.Array_Add` (`self.StreamedLevels`) NewLevel)
  (if (> (`KismetArrayLibrary.Array_Length` (`self.StreamedLevels`)) 3)
    (`LevelStreaming.SetIsRequestingUnloadAndRemoval` (`|GetArrayItem` (`self.StreamedLevels`)) true)
    (`KismetArrayLibrary.Array_Remove` (`self.StreamedLevels`))
    (`/Engine/EditorBlueprintResources/StandardMacros.Gate` true :!label _label
      (:`Exit`
        (`GameplayStatics.UnloadStreamLevel` "FirstMap")))))

(event `Unlock`
  (goto _label :!via `Open`))

(event `AddForestManager`
  (params (NewManager :type "/Game/Blueprints/Gamemode/ForestManager Object Reference"))
  (`KismetArrayLibrary.Array_Add` (`self.ForestManagers`) NewManager))

(event `self.ReceiveBeginPlay`
  (bind _asbp_player_controller (cast `/Game/Blueprints/Player/BP_PlayerController` (`GameplayStatics.GetPlayerController` 0)))
  (`/Game/Blueprints/Player/BP_PlayerController.RespawnPawn` _asbp_player_controller))

(fn `UserConstructionScript`)