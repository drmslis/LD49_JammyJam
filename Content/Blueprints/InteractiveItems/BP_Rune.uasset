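; BP_Rune is a collectible rune item that spins in the world until activated.
; Tick yaws its mesh at a constant, frame-rate-independent speed.
; On ItemActivation it casts to BP_PlayerController, passes its item type name and texture to UpdateInventory, then destroys itself.
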(event `self.ItemActivation`
  (bind _asbp_player_controller (cast `/Game/Blueprints/Player/BP_PlayerController` (`GameplayStatics.GetPlayerController` 0)))
  (`/Game/Blueprints/Player/BP_PlayerController.UpdateInventory` _asbp_player_controller (`KismetTextLibrary.Conv_StringToText` (`|GetEnumeratorNameAsString` (`self.ItemType`))) (`self.Texture`))
  (`self.K2_DestroyActor`))

(event `self.ReceiveTick`
  (params (DeltaSeconds :type "Float (single-precision)"))
  (`SceneComponent.K2_AddWorldRotation` (`self.Mesh`) (`KismetMathLibrary.MakeRotator` 0.0 0.0 (* DeltaSeconds 100.0)) false false))

(fn `UserConstructionScript`
  (`parent.UserConstructionScript`))