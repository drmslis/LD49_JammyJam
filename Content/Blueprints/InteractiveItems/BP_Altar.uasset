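; Interactive altar where the player places offerings from the inventory and, once none are missing, can summon BP_Leshiy at a set spawn point.
; A wide collider creates the hold-to-interact widget, while a close collider shows it and gates input, with a delay and polled timer driving the hold progress.
; BP_PlayerController checks and places offerings, ShowItem reveals the Rune, Eye or Mushroom, and a second gate arms the summon for a later hold.
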(event `self.ReceiveBeginPlay`
  (`parent.ReceiveBeginPlay`)
  (for _array_element (`SceneComponent.GetChildrenComponents` (`self.Mesh`) false)
    (bind _aschild_actor_component (cast `ChildActorComponent` _array_element))
    (`KismetArrayLibrary.Array_Add` (`self.ChildActors`) (make `/Game/Data/OnAltarSlots` (`KismetSystemLibrary.GetObjectName` _aschild_actor_component) _aschild_actor_component))))

(event `InputAction|Interact`
  (params (Key :type "Key Structure"))
  (:`Pressed`
    (set `self.bIsHeld` true)
    (`/Engine/EditorBlueprintResources/StandardMacros.Gate` true :!label _label
      (:`Exit`
        (`|ExecutionSequence`
          (:`then_0`
            (`KismetSystemLibrary.RetriggerableDelay` (`self.TimeToHold`))
            (if (`self.bIsHeld`)
              ;[1 1 1] do smth after timer
              (bind _asbp_player_controller (cast `/Game/Blueprints/Player/BP_PlayerController` (`GameplayStatics.GetPlayerController` 0)))
              (if (== (`KismetArrayLibrary.Array_Length` (`/Game/Blueprints/Player/BP_PlayerController.Inventory` _asbp_player_controller)) 0)
                (`/Game/UI/HoldEWidget.SetText` (`self.Hold EWidget`) "Looks like i need bring some items here")
                (else
                  (bind _asbp_player_controller_2 (cast `/Game/Blueprints/Player/BP_PlayerController` (`GameplayStatics.GetPlayerController` 0)))
                  (bind _isneedsmthelse (`/Game/Blueprints/Player/BP_PlayerController.CheckAllOfferings` _asbp_player_controller_2))
                  (if _isneedsmthelse
                    (`/Game/Blueprints/Player/BP_PlayerController.PlaceOnTheAltar` _asbp_player_controller_2 self)
                    (bind _asbp_player_controller_3 (cast `/Game/Blueprints/Player/BP_PlayerController` (`GameplayStatics.GetPlayerController` 0)))
                    (bind _isneedsmthelse_2 (`/Game/Blueprints/Player/BP_PlayerController.CheckAllOfferings` _asbp_player_controller_3))
                    (if _isneedsmthelse_2
                      (`/Game/UI/HoldEWidget.SetText` (`self.Hold EWidget`) "Looks like you need something else...")
                      (else
                        (`/Game/UI/HoldEWidget.SetText` (`self.Hold EWidget`) "You can summon Leshiy! Beware!")
                        (goto _label_2 :!via `Open`)))
                    (else
                      (`/Engine/EditorBlueprintResources/StandardMacros.Gate` true :!label _label_2
                        (:`Exit`
                          (`self.SpawnLeshiy`)
                          (`/Game/UI/HoldEWidget.SetText` (`self.Hold EWidget`) "!!!")
                          (goto _label_2 :!via `Close`)))))))))
          (:`then_1`
            (`self.StartTimer`)
            (`self.Update Timer`))))))
  (:`Released`
    (set `self.bIsHeld` false)))

(event `self.CloseRangeCollider.OnComponentBeginOverlap`
  (params (OverlappedComponent :type "PrimitiveComponent Object Reference") (OtherActor :type "Actor Object Reference") (OtherComp :type "PrimitiveComponent Object Reference") (OtherBodyIndex :type Integer) (bFromSweep :type Boolean) (SweepResult :type "HitResult Structure (by ref)"))
  (cast `/Game/Blueprints/Player/BP_Player` OtherActor)
  (`self.EnableInput` (`GameplayStatics.GetPlayerController` 0))
  (`/Engine/EditorBlueprintResources/StandardMacros.IsValid` (`self.Hold EWidget`)
    (:`Is Valid`
      (`Widget.SetVisibility` (`self.Hold EWidget`) "Visible")
      (goto _label :!via `Open`))))

(event `StopTimer`
  (`KismetSystemLibrary.K2_PauseTimerHandle` (stale `StartTimer` _returnvalue)))

(event `StartTimer`
  (bind _returnvalue (`KismetSystemLibrary.K2_SetTimerDelegate` (delegate `StartTimer`) (`self.TimeToHold`))))

(event `ShowItem`
  (params (NewParam :type String))
  (`KismetSystemLibrary.PrintString` NewParam)
  (switch `string` NewParam
    (:`Rune`
      (`SceneComponent.SetVisibility` (`self.Rune`) true false))
    (:`Eye`
      (`SceneComponent.SetVisibility` (`self.Eye`) true false))
    (:`Mushroom`
      (`SceneComponent.SetVisibility` (`self.Mushroom`) true false))))

(event `self.CloseRangeCollider.OnComponentEndOverlap`
  (params (OverlappedComponent :type "PrimitiveComponent Object Reference") (OtherActor :type "Actor Object Reference") (OtherComp :type "PrimitiveComponent Object Reference") (OtherBodyIndex :type Integer))
  (cast `/Game/Blueprints/Player/BP_Player` OtherActor)
  (`self.EnableInput` (`GameplayStatics.GetPlayerController` 0))
  (`/Engine/EditorBlueprintResources/StandardMacros.IsValid` (`self.Hold EWidget`)
    (:`Is Valid`
      (`Widget.SetVisibility` (`self.Hold EWidget`) "Collapsed")
      (goto _label :!via `Close`))))

(event `Update Timer`
  (if (`self.bIsHeld`)
    (`/Game/UI/HoldEWidget.SetElapsedTime` (`self.Hold EWidget`) (`KismetSystemLibrary.K2_GetTimerElapsedTimeHandle` (stale `StartTimer` _returnvalue)))
    (`KismetSystemLibrary.Delay` 0.1)
    (`self.Update Timer`)
    (else
      (`self.StopTimer`)
      (`/Game/UI/HoldEWidget.SetElapsedTime` (`self.Hold EWidget`) 0.0))))

(event `SpawnLeshiy`
  (bind _leshiyspawn (`self.LeshiySpawn`))
  (`/Engine/EditorBlueprintResources/StandardMacros.IsValid` (`self.LeshiySpawn`)
    (:`Is Valid`
      (`|SpawnActorFromClass` "/Game/Blueprints/Enemies/BP_Leshiy.BP_Leshiy_C" (`KismetMathLibrary.MakeTransform` (`self.K2_GetActorLocation` _leshiyspawn) (`self.K2_GetActorRotation` _leshiyspawn)) "AdjustIfPossibleButAlwaysSpawn" "OverrideRootScale" null null))
    (:`Is Not Valid`
      (`KismetSystemLibrary.PrintString` "SPAWN POINT NOT SET" true true (struct :`R` 1.0 :`B` 0.039114 :`A` 1.0)))))

(event `self.WideRangeCollider.OnComponentBeginOverlap`
  (params (OverlappedComponent :type "PrimitiveComponent Object Reference") (OtherActor :type "Actor Object Reference") (OtherComp :type "PrimitiveComponent Object Reference") (OtherBodyIndex :type Integer) (bFromSweep :type Boolean) (SweepResult :type "HitResult Structure (by ref)"))
  (bind _returnvalue (`|CreateWidget` "/Game/UI/HoldEWidget.HoldEWidget_C"))
  (bind _output_get (set `self.Hold EWidget` _returnvalue))
  (`/Game/UI/HoldEWidget.SetText` _output_get (`self.TextToHold`))
  (`/Game/UI/HoldEWidget.SetTimeToHold` (`self.Hold EWidget`) (`self.TimeToHold`))
  (`UserWidget.AddToViewport` (`self.Hold EWidget`) 0)
  (`Widget.SetVisibility` (`self.Hold EWidget`) "Collapsed")
  (bind _asbp_player_controller (cast `/Game/Blueprints/Player/BP_PlayerController` (`GameplayStatics.GetPlayerController` 0)))
  (if (== (`KismetArrayLibrary.Array_Length` (`/Game/Blueprints/Player/BP_PlayerController.Inventory` _asbp_player_controller)) 0)
    (`/Game/UI/HoldEWidget.SetText` (`self.Hold EWidget`) "...")
    (else
      (`/Game/UI/HoldEWidget.SetText` (`self.Hold EWidget`) "Place your offerings on altar, mortal"))))

(event `self.WideRangeCollider.OnComponentEndOverlap`
  (params (OverlappedComponent :type "PrimitiveComponent Object Reference") (OtherActor :type "Actor Object Reference") (OtherComp :type "PrimitiveComponent Object Reference") (OtherBodyIndex :type Integer))
  (`/Engine/EditorBlueprintResources/StandardMacros.IsValid` (`self.Hold EWidget`)
    (:`Is Valid`
      (`Widget.RemoveFromParent` (`self.Hold EWidget`)))))

(fn `CheckAllOfferings`
  (params (Array :type "Array of /Game/Data/ItemSlot Structure"))
  (returns (IsNeedSmthElse :type Boolean))
  (locals (IsNeed :type Boolean :default true))
  (for _array_element Array
    (if (`.IsOnAltar_5_3FAF551E497A7D9E0211AE8AA097AC60` (break `/Game/Data/ItemSlot` _array_element))
      (set `self.Need smth` false)
      (else
        (set `self.Need smth` true)
        (break))))
  (return (`local.IsNeed`)))

(fn `UserConstructionScript`
  (`parent.UserConstructionScript`))