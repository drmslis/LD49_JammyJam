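; Test pickup item that the player holds Interact on to collect, destroying itself if still held when TimeToHold expires.
; The wide collider creates and removes a HoldEWidget prompt, while the close collider toggles its visibility and the Gate that admits the press.
; A retriggerable delay decides the pickup.
; A separate timer supplies elapsed time to the widget through a self-calling 0.1-second update that resets on release.
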(event `self.ReceiveBeginPlay`
  (`parent.ReceiveBeginPlay`))

(event `InputAction|Interact`
  (params (Key :type "Key Structure"))
  (:`Pressed`
    (set `self.bIsHeld` true)
    (`/Engine/EditorBlueprintResources/StandardMacros.Gate` true :!label _label
      (:`Exit`
        (`|ExecutionSequence`
          (:`then_0`
            (`KismetSystemLibrary.RetriggerableDelay` (`self.TimeToHold`))
            (if (`self.bIsHeld`)
              ;[1 1 1] do smth after timer
              (`self.K2_DestroyActor`)))
          (:`then_1`
            (`self.StartTimer`)
            (`self.Update Timer`))))))
  (:`Released`
    (set `self.bIsHeld` false)))

(event `self.CloseRangeCollider.OnComponentBeginOverlap`
  (params (OverlappedComponent :type "PrimitiveComponent Object Reference") (OtherActor :type "Actor Object Reference") (OtherComp :type "PrimitiveComponent Object Reference") (OtherBodyIndex :type Integer) (bFromSweep :type Boolean) (SweepResult :type "HitResult Structure (by ref)"))
  (`self.EnableInput` (`GameplayStatics.GetPlayerController` 0))
  (`/Engine/EditorBlueprintResources/StandardMacros.IsValid` (`self.Hold EWidget`)
    (:`Is Valid`
      (`Widget.SetVisibility` (`self.Hold EWidget`) "Visible")
      (goto _label :!via `Open`))))

(event `StopTimer`
  (`KismetSystemLibrary.K2_PauseTimerHandle` (stale `StartTimer` _returnvalue)))

(event `StartTimer`
  (bind _returnvalue (`KismetSystemLibrary.K2_SetTimerDelegate` (delegate `StartTimer`) (`self.TimeToHold`))))

(event `self.CloseRangeCollider.OnComponentEndOverlap`
  (params (OverlappedComponent :type "PrimitiveComponent Object Reference") (OtherActor :type "Actor Object Reference") (OtherComp :type "PrimitiveComponent Object Reference") (OtherBodyIndex :type Integer))
  (`self.EnableInput` (`GameplayStatics.GetPlayerController` 0))
  (`/Engine/EditorBlueprintResources/StandardMacros.IsValid` (`self.Hold EWidget`)
    (:`Is Valid`
      (`Widget.SetVisibility` (`self.Hold EWidget`) "Collapsed")
      (goto _label :!via `Close`))))

(event `Update Timer`
  (if (`self.bIsHeld`)
    (`/Game/UI/HoldEWidget.SetElapsedTime` (`self.Hold EWidget`) (`KismetSystemLibrary.K2_GetTimerElapsedTimeHandle` (stale `StartTimer` _returnvalue)))
    (`KismetSystemLibrary.Delay` 0.1)
    (`self.Update Timer`)
    (else
      (`self.StopTimer`)
      (`/Game/UI/HoldEWidget.SetElapsedTime` (`self.Hold EWidget`) 0.0))))

(event `self.WideRangeCollider.OnComponentBeginOverlap`
  (params (OverlappedComponent :type "PrimitiveComponent Object Reference") (OtherActor :type "Actor Object Reference") (OtherComp :type "PrimitiveComponent Object Reference") (OtherBodyIndex :type Integer) (bFromSweep :type Boolean) (SweepResult :type "HitResult Structure (by ref)"))
  (bind _returnvalue (`|CreateWidget` (`self.HoldEWidget`)))
  (bind _ashold_ewidget (cast `/Game/UI/HoldEWidget` _returnvalue))
  (bind _output_get (set `self.Hold EWidget` _ashold_ewidget))
  (`/Game/UI/HoldEWidget.SetText` _output_get (`self.TextToHold`))
  (`/Game/UI/HoldEWidget.SetTimeToHold` (`self.Hold EWidget`) (`self.TimeToHold`))
  (`UserWidget.AddToViewport` (`self.Hold EWidget`) 0)
  (`Widget.SetVisibility` (`self.Hold EWidget`) "Collapsed"))

(event `self.WideRangeCollider.OnComponentEndOverlap`
  (params (OverlappedComponent :type "PrimitiveComponent Object Reference") (OtherActor :type "Actor Object Reference") (OtherComp :type "PrimitiveComponent Object Reference") (OtherBodyIndex :type Integer))
  (`/Engine/EditorBlueprintResources/StandardMacros.IsValid` (`self.Hold EWidget`)
    (:`Is Valid`
      (`Widget.RemoveFromParent` (`self.Hold EWidget`)))))

(fn `UserConstructionScript`
  (`parent.UserConstructionScript`))