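; BP_Eye is a collectible eye item, built on an interactive-item parent class, that the player picks up into the inventory.
; On ItemActivation it passes its ItemType name and Texture to BP_PlayerController's UpdateInventory, then destroys itself.
; The big-collider overlap overrides only call the parent, with the begin call passing empty text and zero hold time instead of its inputs.
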(event `self.ItemActivation`
  (bind _asbp_player_controller (cast `/Game/Blueprints/Player/BP_PlayerController` (`GameplayStatics.GetPlayerController` 0)))
  (`/Game/Blueprints/Player/BP_PlayerController.UpdateInventory` _asbp_player_controller (`KismetTextLibrary.Conv_StringToText` (`|GetEnumeratorNameAsString` (`self.ItemType`))) (`self.Texture`))
  (`self.K2_DestroyActor`))

(fn `EndOverlapBigCollider`
  (`parent.EndOverlapBigCollider`))

(fn `OverlapBigCollider`
  (params (InText :type Text) (MaxTimeToHold :type "Float (double-precision)"))
  (`parent.OverlapBigCollider` "" 0.0))

(fn `UserConstructionScript`
  (`parent.UserConstructionScript`))