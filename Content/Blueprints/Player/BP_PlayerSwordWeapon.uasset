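; Player sword weapon that applies damage to actors other than its owner when they overlap its WeaponCollider.
; A DoOnce gate limits damage to one hit at a time, and a named timer resets it after ReactivationTimer, so the cooldown is shared across all targets.
; ColliderActivate and ColliderDeactivate open and close the hit window by applying the Trigger collision profile or disabling collision.
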(event `self.WeaponCollider.OnComponentBeginOverlap`
  (params (OverlappedComponent :type "PrimitiveComponent Object Reference") (OtherActor :type "Actor Object Reference") (OtherComp :type "PrimitiveComponent Object Reference") (OtherBodyIndex :type Integer) (bFromSweep :type Boolean) (SweepResult :type "HitResult Structure (by ref)"))
  (if (!= OtherActor (`self.GetOwner`))
    (`/Engine/EditorBlueprintResources/StandardMacros.DoOnce` false :!label _label
      (:`Completed`
        (`GameplayStatics.ApplyDamage` OtherActor (`self.Damage`))
        (`KismetSystemLibrary.K2_SetTimer` null "Re-Acttivate " (`self.Reactivation Timer`))))))

(event `Re-Acttivate`
  (goto _label :!via `Reset`))

(event `ColliderActivate`
  (`PrimitiveComponent.SetCollisionProfileName` (`self.WeaponCollider`) "Trigger" true))

(event `Collider Deactivate`
  (`PrimitiveComponent.SetCollisionEnabled` (`self.WeaponCollider`) "NoCollision"))

(fn `UserConstructionScript`
  (`parent.UserConstructionScript`))