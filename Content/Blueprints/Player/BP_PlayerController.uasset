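; Player controller that owns the item inventory, main HUD and respawning for BP_Player.
; Respawning spawns a pawn at the first PlayerStart, possesses it and refreshes the UI.
; Collected items are flagged and shown when placed on an altar, while CheckAllOfferings reports whether offerings are still outstanding for the summon.
; Input drives attack, control help and alternating flashlight/sword toggles, and Tick prints inventory debug text.
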(event `self.ReceiveBeginPlay`)

(event `self.ReceiveTick`
  (params (DeltaSeconds :type "Float (single-precision)"))
  (for _array_element (`self.Inventory`)
    (`KismetSystemLibrary.PrintString` (`KismetTextLibrary.Conv_TextToString` (`|FormatText` "{Name} : {IsPlaced}" (break `/Game/Data/ItemSlot` _array_element) (`.IsOnAltar_5_3FAF551E497A7D9E0211AE8AA097AC60` (break `/Game/Data/ItemSlot` _array_element)))) true true (struct :`G` 0.66 :`B` 1.0 :`A` 1.0) 0.0))
  (bind _isneedsmthelse (`self.CheckAllOfferings`))
  (`KismetSystemLibrary.PrintString` (`KismetStringLibrary.Conv_BoolToString` _isneedsmthelse) true true (struct :`G` 0.66 :`B` 1.0 :`A` 1.0) 0.0))

(event `RespawnPawn`
  (bind _outactors (`GameplayStatics.GetAllActorsOfClass` "/Script/Engine.PlayerStart"))
  (bind _output (`|GetArrayItem` _outactors))
  (bind _returnvalue (`|SpawnActorFromClass` "/Game/Blueprints/Player/BP_Player.BP_Player_C" (`KismetMathLibrary.MakeTransform` (`self.K2_GetActorLocation` _output) (`self.K2_GetActorRotation` _output)) "AdjustIfPossibleButAlwaysSpawn" "OverrideRootScale" null null))
  (bind _output_get (set `self.Possessed Pawn` _returnvalue))
  (`self.Possess` self _output_get))

(event `self.ReceivePossess`
  (params (PossessedPawn :type "Pawn Object Reference"))
  (bind _asbp_player (cast `/Game/Blueprints/Player/BP_Player` (`self.Possessed Pawn`) :!pure true))
  (set `self.Possessed Pawn` PossessedPawn)
  (`/Engine/EditorBlueprintResources/StandardMacros.IsValid` (`self.MainUI`)
    (:`Is Valid`
      _)
    (:`Is Not Valid`
      (bind _returnvalue (`|CreateWidget` "/Game/UI/MainUI.MainUI_C"))
      (bind _output_get (set `self.MainUI` _returnvalue))
      (`UserWidget.AddToViewport` _output_get 0)))
  (`Widget.SetVisibility` (`self.MainUI`) "HitTestInvisible")
  (`/Game/Blueprints/Player/BP_Player.Respawn` _asbp_player)
  (`/Game/Blueprints/Player/BP_Player.UpdateHPBar` _asbp_player)
  (`self.EnableInput` self))

(event `HPBarHandle`
  (params (InPercent :type "Float (double-precision)"))
  (`/Game/UI/MainUI.SetHP` (`self.MainUI`) InPercent))

(event `DeathScreenHandle`
  (`/Engine/EditorBlueprintResources/StandardMacros.IsValid` (`self.MainUI`)
    (:`Is Valid`
      (`Widget.SetVisibility` (`self.MainUI`) "Collapsed"))))

(event `UpdateInventory`
  (params (`Item Name` :type Text) (Icon :type "Texture2D Object Reference"))
  (`KismetArrayLibrary.Array_AddUnique` (`self.Inventory`) (make `/Game/Data/ItemSlot` `Item Name` false Icon))
  (`/Game/UI/MainUI.UpdateSlots` (`self.MainUI`)))

(event `PlaceOnTheAltar`
  (params (Altar :type "/Game/Blueprints/InteractiveItems/BP_Altar Object Reference"))
  (set `self.Altar` Altar)
  (for (_array_element _array_index) (`self.Inventory`)
    (bind (_itemname _isonaltar _icon) (break `/Game/Data/ItemSlot` _array_element))
    (if (not _isonaltar)
      (`|VariableSetRef` (`|GetArrayItem` (`self.Inventory`) _array_index) (make `/Game/Data/ItemSlot` _itemname true _icon))
      (`/Game/Blueprints/InteractiveItems/BP_Altar.ShowItem` (`self.Altar`) (`KismetTextLibrary.Conv_TextToString` _itemname))))
  (`/Game/UI/MainUI.UpdateSlots` (`self.MainUI`)))

(event `InputAction|F1 - controls`
  (params (Key :type "Key Structure"))
  (:`Pressed`
    (`/Engine/EditorBlueprintResources/StandardMacros.FlipFlop`
      (:`A`
        (`/Game/UI/MainUI.SetControlHelpVisibility` (`self.MainUI`) "Visible"))
      (:`B`
        (`/Game/UI/MainUI.SetControlHelpVisibility` (`self.MainUI`) "Collapsed")))))

(event `InputAction|Flashlight`
  (params (Key :type "Key Structure"))
  (bind _asbp_player (cast `/Game/Blueprints/Player/BP_Player` (`self.Possessed Pawn`) :!pure true))
  (:`Pressed`
    (`/Engine/EditorBlueprintResources/StandardMacros.FlipFlop`
      (:`A`
        (`/Game/Blueprints/Player/BP_Player.FlashLight Toggle` _asbp_player))
      (:`B`
        (`/Game/Blueprints/Player/BP_Player.SwordToggle` _asbp_player)))))

(event `AddItem`
  (params (ItemName :type Text) (Icon :type "Texture2D Object Reference"))
  (`KismetArrayLibrary.Array_Add` (`self.Inventory`) (make `/Game/Data/ItemSlot` ItemName false Icon)))

(event `InputAction|Attack`
  (params (Key :type "Key Structure"))
  (:`Pressed`
    (`/Game/Blueprints/Player/BP_Player.AttackLogic` (cast `/Game/Blueprints/Player/BP_Player` (`self.Possessed Pawn`) :!pure true))))

(event `InputAction|Block`
  (params (Key :type "Key Structure")))

(event `InputAction|Interact`
  (params (Key :type "Key Structure")))

(event `InputAction|Inventory\\Map`
  (params (Key :type "Key Structure")))

(event `InputAction|EscMenu`
  (params (Key :type "Key Structure")))

(fn `CheckAllOfferings`
  (returns (IsNeedSmthElse :type Boolean))
  (locals (IsNeed :type Boolean))
  (bind _inventory (`self.Inventory`))
  (if (< (`KismetArrayLibrary.Array_Length` _inventory) (`self.ItemsNeededForSummon`))
    (return true)
    (else
      (for _array_element _inventory
        (if (`.IsOnAltar_5_3FAF551E497A7D9E0211AE8AA097AC60` (break `/Game/Data/ItemSlot` _array_element))
          (set `local.IsNeed` false)
          (else
            (set `local.IsNeed` true)
            (break))))
      (return (`local.IsNeed`)))))

(fn `UserConstructionScript`)